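; BP_Car is a player-drivable sports car Blueprint built on Chaos wheeled vehicle movement.
; BeginPlay adds the vehicle Enhanced Input mapping context to the first player controller's subsystem.
; Input actions feed throttle, steering and handbrake to the movement component, with brake driven by the negated forward/backward axis and inputs reset on release.
; Camera input adds controller yaw and pitch.
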(event Input|EnhancedActionEvents|EnhancedInputActionIA_CameraControls
  (params (ActionValue :type Vector%202D%20Structure) (ElapsedSeconds :type Float%20%28double-precision%29) (TriggeredSeconds :type Float%20%28double-precision%29) (InputAction :type Input%20Action%20Object%20Reference :default "/Game/Configurations/Inputs/IA_CameraControls.IA_CameraControls"))
  (bind (_x _y) (Math|Vector2D|BreakVector2D ActionValue))
  (Pawn|Input|AddControllerYawInput _x)
  (Pawn|Input|AddControllerPitchInput _y))

(event Input|EnhancedActionEvents|EnhancedInputActionIA_ForwardBackward
  (params (ActionValue :type Float%20%28double-precision%29) (ElapsedSeconds :type Float%20%28double-precision%29) (TriggeredSeconds :type Float%20%28double-precision%29) (InputAction :type Input%20Action%20Object%20Reference :default "/Game/Configurations/Inputs/IA_ForwardBackward.IA_ForwardBackward"))
  (:Triggered
    (Class|ChaosVehicleMovementComponent|SetThrottleInput (Variables|Default|GetChaosWheeledVehicleMovement) ActionValue)
    (Class|ChaosVehicleMovementComponent|SetBrakeInput (Variables|Default|GetChaosWheeledVehicleMovement) (* ActionValue -1.0)))
  (:Completed
    (Class|ChaosVehicleMovementComponent|SetThrottleInput (Variables|Default|GetChaosWheeledVehicleMovement) 0.0)
    (Class|ChaosVehicleMovementComponent|SetBrakeInput (Variables|Default|GetChaosWheeledVehicleMovement) (* 0.0 -1.0))))

(event Input|EnhancedActionEvents|EnhancedInputActionIA_Handbrake
  (params (ActionValue :type Boolean) (ElapsedSeconds :type Float%20%28double-precision%29) (TriggeredSeconds :type Float%20%28double-precision%29) (InputAction :type Input%20Action%20Object%20Reference :default "/Game/Configurations/Inputs/IA_Handbrake.IA_Handbrake"))
  (:Started
    (Class|ChaosVehicleMovementComponent|SetHandbrakeInput (Variables|Default|GetChaosWheeledVehicleMovement) true))
  (:Completed
    (Class|ChaosVehicleMovementComponent|SetHandbrakeInput (Variables|Default|GetChaosWheeledVehicleMovement) false)))

(event Input|EnhancedActionEvents|EnhancedInputActionIA_LeftRight
  (params (ActionValue :type Float%20%28double-precision%29) (ElapsedSeconds :type Float%20%28double-precision%29) (TriggeredSeconds :type Float%20%28double-precision%29) (InputAction :type Input%20Action%20Object%20Reference :default "/Game/Configurations/Inputs/IA_LeftRight.IA_LeftRight"))
  (:Triggered
    (Class|ChaosVehicleMovementComponent|SetSteeringInput (Variables|Default|GetChaosWheeledVehicleMovement) ActionValue))
  (:Completed
    (Class|ChaosVehicleMovementComponent|SetSteeringInput (Variables|Default|GetChaosWheeledVehicleMovement) 0.0)))

(event EventBeginPlay
  (Input|AddMappingContext (PlayerController|LocalPlayerSubsystems|GetEnhancedInputLocalPlayerSubsystem (Game|GetPlayerController 0)) "/Game/Configurations/Inputs/IMC_Vehicles.IMC_Vehicles" 0 "(bIgnoreAllPressedKeysUntilRelease=True,bForceImmediately=False,bNotifyUserSettings=False)"))

(event Collision|EventActorBeginOverlap
  (params (OtherActor :type Actor%20Object%20Reference)))

(event EventTick
  (params (DeltaSeconds :type Float%20%28single-precision%29)))

(fn ConstructionScript)